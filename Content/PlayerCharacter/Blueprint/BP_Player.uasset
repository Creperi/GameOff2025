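; Player character Blueprint handling third-person movement, swimming and opening the pause menu.
; On possession it adds the Enhanced Input mapping context for move, turn and jump; forward movement follows full control rotation while swimming, yaw only otherwise.
; Start/Stop swimming events toggle WaterVolume on the current physics volume and mirror it in IsSwimming, with a small upward launch on start.
; P shows a cached pause widget, switches to UI-only input and pauses the game.
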(event `Key|P`
  (params (Key :type "Key Structure"))
  (bind _returnvalue (`GameplayStatics.GetPlayerController` 0))
  (bind _pause_menu_reference (`self.Pause Menu Reference`))
  (:`Pressed`
    (`/Engine/EditorBlueprintResources/StandardMacros.IsValid` (`self.Pause Menu Reference`)
      (:`Is Valid`
        (set `PlayerController.bShowMouseCursor` true _returnvalue))
      (:`Is Not Valid`
        (bind _returnvalue_2 (`|CreateWidget` "/Game/UI/PauseMenu.PauseMenu_C"))
        (set `self.Pause Menu Reference` _returnvalue_2)))
    (`WidgetBlueprintLibrary.SetInputMode_UIOnlyEx` _returnvalue _pause_menu_reference)
    (`UserWidget.AddToViewport` _pause_menu_reference 0)
    (`GameplayStatics.SetGamePaused` true)))

(event `self.ReceivePossessed`
  (params (NewController :type "Controller Object Reference"))
  (bind _asplayer_controller (cast `PlayerController` NewController))
  (`EnhancedInputSubsystemInterface.AddMappingContext` (pcsubsystem `EnhancedInputLocalPlayerSubsystem` _asplayer_controller) "/Game/PlayerCharacter/Input/IM_ThirdPerson.IM_ThirdPerson" 0 (struct)))

(event `EnhancedInput|/Game/PlayerCharacter/Input/IA_Moveforward`
  (params (ActionValue :type "Float (double-precision)") (ElapsedSeconds :type "Float (double-precision)") (TriggeredSeconds :type "Float (double-precision)") (InputAction :type "InputAction Object Reference" :default "/Game/PlayerCharacter/Input/IA_Moveforward.IA_Moveforward"))
  (:`Triggered`
    (if (`self.isSwimming`)
      (`self.AddMovementInput` (`KismetMathLibrary.GetForwardVector` (`self.GetControlRotation`)) ActionValue)
      (else
        (`self.AddMovementInput` (`KismetMathLibrary.GetForwardVector` (`KismetMathLibrary.MakeRotator` 0.0 0.0 (.yaw (`self.GetControlRotation`)))) ActionValue)))))

(event `EnhancedInput|/Game/PlayerCharacter/Input/IA_Moveright`
  (params (ActionValue :type "Float (double-precision)") (ElapsedSeconds :type "Float (double-precision)") (TriggeredSeconds :type "Float (double-precision)") (InputAction :type "InputAction Object Reference" :default "/Game/PlayerCharacter/Input/IA_Moveright.IA_Moveright"))
  (:`Triggered`
    (`self.AddMovementInput` (`KismetMathLibrary.GetRightVector` (`KismetMathLibrary.MakeRotator` 0.0 0.0 (.yaw (`self.GetControlRotation`)))) ActionValue)))

(event `EnhancedInput|/Game/PlayerCharacter/Input/IA_Turn`
  (params (ActionValue :type "Float (double-precision)") (ElapsedSeconds :type "Float (double-precision)") (TriggeredSeconds :type "Float (double-precision)") (InputAction :type "InputAction Object Reference" :default "/Game/PlayerCharacter/Input/IA_Turn.IA_Turn"))
  (:`Triggered`
    (`self.AddControllerYawInput` ActionValue)))

(event `EnhancedInput|/Game/PlayerCharacter/Input/IA_Jump`
  (params (ActionValue :type Boolean) (ElapsedSeconds :type "Float (double-precision)") (TriggeredSeconds :type "Float (double-precision)") (InputAction :type "InputAction Object Reference" :default "/Game/PlayerCharacter/Input/IA_Jump.IA_Jump"))
  (:`Triggered`
    (`self.Jump`)))

(event `Start swimming`
  (`self.LaunchCharacter` (* (`KismetMathLibrary.GetUpVector` (`self.K2_GetActorRotation`)) 2.0))
  (bind _output_get (set `PhysicsVolume.bWaterVolume` true (`MovementComponent.GetPhysicsVolume` (`self.CharacterMovement`))))
  (set `self.isSwimming` _output_get))

(event `Stop swimming`
  (bind _output_get (set `PhysicsVolume.bWaterVolume` false (`MovementComponent.GetPhysicsVolume` (`self.CharacterMovement`))))
  (set `self.isSwimming` _output_get))

(fn `UserConstructionScript`)